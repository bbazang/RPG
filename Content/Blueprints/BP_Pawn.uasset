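; BP_Pawn is a player-flown aircraft pawn that constantly moves forward and fires rockets.
; BeginPlay adds the IMC_Input Enhanced Input mapping context, and Tick drives forward movement while spinning the left and right propellers.
; The pitchandroll action feeds controller pitch and roll, and Fire spawns a BP_Rocket at the Arrow component's transform.
; The legacy Pitch and Roll axis events are empty.
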(event Input|EnhancedActionEvents|EnhancedInputActionpitchandroll
  (params (ActionValue :type Vector%202D%20Structure) (ElapsedSeconds :type Float%20%28double-precision%29) (TriggeredSeconds :type Float%20%28double-precision%29) (InputAction :type Input%20Action%20Object%20Reference :default "/Game/Blueprints/Input/pitchandroll.pitchandroll"))
  (:Triggered
    (Pawn|Input|AddControllerPitchInput (.x ActionValue))
    (Pawn|Input|AddControllerRollInput (.y ActionValue))))

(event EventBeginPlay
  (Utilities|IsValid (Game|GetPlayerController 0)
    (:Is%20Valid
      (Input|AddMappingContext (PlayerController|LocalPlayerSubsystems|GetEnhancedInputLocalPlayerSubsystem (Game|GetPlayerController 0)) "/Game/Blueprints/Input/IMC_Input.IMC_Input" 0 "(bIgnoreAllPressedKeysUntilRelease=True,bForceImmediately=False)"))))

(event EventTick
  (params (DeltaSeconds :type Float%20%28single-precision%29))
  ;[1 1 1] 무브먼트 이동
  (Pawn|Input|AddMovementInput (Transformation|GetActorForwardVector) 1.0 false)
  ;[1 1 1] 왼쪽 프로펠러 회전
  (Transformation|AddLocalRotation (Variables|Default|GetLeft) (* (Variables|속력|GetPropellerRotationSpeed) (Utilities|Time|GetWorldDeltaSeconds)) false false)
  ;[1 1 1] 오른쪽 프로펠러 회전
  (Transformation|AddLocalRotation (Variables|Default|GetRight) (* (Variables|속력|GetPropellerRotationSpeed) (Utilities|Time|GetWorldDeltaSeconds)) false false))

(event Input|ActionEvents|InputActionFire
  (params (Key :type Key%20Structure :default "None"))
  ;[1 1 1] 미사일 발사
  (:Pressed
    (Game|SpawnActorfromClass "/Game/Blueprints/BP_Rocket.BP_Rocket_C" (Transformation|GetWorldTransform (Variables|Default|GetArrow)) "Undefined" 0 0)))

(event Input|AxisEvents|InputAxisPitch
  (params (AxisValue :type Float%20%28single-precision%29)))

(event Input|AxisEvents|InputAxisRoll
  (params (AxisValue :type Float%20%28single-precision%29)))

(fn ConstructionScript)